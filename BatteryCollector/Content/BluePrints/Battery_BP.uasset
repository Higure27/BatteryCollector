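; Battery pickup actor that plays a collection effect when the player collects it.
; On WasCollected it adds an audio component and attaches an electric arc beam emitter to the pickup mesh.
; The beam's target follows the player character's spine socket, refreshed by a short delay loop, until the actor destroys itself after a second.
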(event `self.WasCollected`
  (`AddComponent|NODE_AddAudioComponent-1`)
  (bind _returnvalue (`GameplayStatics.SpawnEmitterAttached` "/Game/ExampleContent/Effects/ParticleSystems/P_electricity_arc.P_electricity_arc" (`self.PickupMesh`) "None" (0.0 0.0 0.0) (struct) (1.0 1.0 1.0) "SnapToTargetIncludingScale"))
  (`ParticleSystemComponent.SetBeamTargetPoint` _returnvalue 0 (`SceneComponent.GetSocketLocation` (`Character.Mesh` (`GameplayStatics.GetPlayerCharacter` 0)) "spine_03") 0 :!label _label)
  (`|ExecutionSequence`
    (:`then_0`
      (`KismetSystemLibrary.Delay` 1.0)
      (`self.K2_DestroyActor`))
    (:`then_1`
      (`KismetSystemLibrary.Delay` 0.1)
      (goto _label))))

(fn `UserConstructionScript`)